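; BP_Building_Mine is a mine building that, once constructed, pulls resources from a nearby deposit into its own stock up to a cap.
; A looping timer started at BeginPlay runs Extract, which takes a fixed amount from the linked deposit.
; When no valid deposit is linked, that tick instead searches the cached resource deposit actors for the nearest within the extraction radius and links it for later ticks.
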(event `Extract`
  (bind _deposit (`self.Deposit`))
  (if (and (`self.bConstructed`) (< (`self.Stock`) (`self.MaxStock`)))
    (`/Engine/EditorBlueprintResources/StandardMacros.IsValid` _deposit
      (:`Is Valid`
        (bind _taken (`/Game/Blueprints/Resources/BP_BaseResource.Take` _deposit (`self.ExtractAmount`)))
        (set `self.Stock` (+ (`self.Stock`) _taken)))
      (:`Is Not Valid`
        (set `self.BestDist` (`self.ExtractRadius`))
        (bind _outactors (`ActorScanner.GetCachedActorsOfClass` "/Game/Blueprints/Resources/BP_ResourceDeposit.BP_ResourceDeposit_C"))
        (for _array_element _outactors
          (bind _returnvalue (`self.GetDistanceTo` self _array_element))
          (if (< _returnvalue (`self.BestDist`))
            (set `self.BestDist` _returnvalue)
            (set `self.Deposit` _array_element)))))))

(event `self.ReceiveBeginPlay`
  (`KismetSystemLibrary.K2_SetTimer` self "Extract" (`self.ExtractInterval`) true))

(fn `UserConstructionScript`
  (`parent.UserConstructionScript`))