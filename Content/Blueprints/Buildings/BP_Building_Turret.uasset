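; Turret building Blueprint that automatically attacks enemy units in range once constructed.
; BeginPlay starts a looping timer at the data's attack cooldown, with a minimum interval, that runs TurretScan.
; Each scan searches cached BP_UnitBase actors for the nearest one of another faction within attack range.
; It hits that unit instantly through TakeHit and draws a brief debug line as the shot visual.
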(event `self.ReceiveBeginPlay`
  (`KismetSystemLibrary.K2_SetTimer` self "TurretScan" (`KismetMathLibrary.FMax` (`/Game/Blueprints/Data/PDA_Building.AttackCooldown` (`self.Data`)) 0.2) true))

(event `TurretScan`
  (bind _turrettarget (`self.TurretTarget`))
  (bind _data (`self.Data`))
  (if (`self.bConstructed`)
    (set `self.TurretTarget` null)
    (set `self.BestDist` (`/Game/Blueprints/Data/PDA_Building.AttackRange` _data))
    (bind _outactors (`ActorScanner.GetCachedActorsOfClass` "/Game/Blueprints/Units/BP_UnitBase.BP_UnitBase_C"))
    (for _array_element _outactors
      (bind _returnvalue (`self.GetDistanceTo` self _array_element))
      (if (and (`|EnumInequality` (`/Game/Blueprints/Units/BP_UnitBase.Faction` _array_element) (`self.Faction`)) (< _returnvalue (`self.BestDist`)))
        (set `self.BestDist` _returnvalue)
        (set `self.TurretTarget` _array_element)))
    (`/Engine/EditorBlueprintResources/StandardMacros.IsValid` _turrettarget
      (:`Is Valid`
        (`KismetSystemLibrary.DrawDebugLine` (+ (`self.K2_GetActorLocation` self) (`KismetMathLibrary.MakeVector` 0.0 0.0 250.0)) (`self.K2_GetActorLocation` _turrettarget) (struct :`R` 1 :`G` 0.3 :`B` 0.1 :`A` 1) 0.15 6.0)
        (`/Game/Blueprints/Units/BP_UnitBase.TakeHit` _turrettarget (`/Game/Blueprints/Data/PDA_Building.AttackDamage` _data) self)))))

(fn `UserConstructionScript`
  (`parent.UserConstructionScript`))