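; Base RTS building actor with selection, ghost placement, timed construction shown by Z scale, damage, and a defeat or victory message when a depot dies.
; TrainUnit charges GM_Default's faction state and queues up to five units on a timer.
; FinishTrain refunds the cost, then re-enters TrainUnit via BypassQueue to charge again and spawn the faction's unit near SpawnPoint.
; Transporters spawned from mines add the mine to their route.
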(event `/Game/Blueprints/BPI_Selectable.Select`
  (params (Selected :type Boolean))
  (`SceneComponent.SetVisibility` (`self.Selection`) Selected false))

(event `SpawnTransporter`
  (bind _returnvalue (`KismetMathLibrary.MakeTransform` (+ (`SceneComponent.K2_GetComponentLocation` (`self.SpawnPoint`)) (`KismetMathLibrary.MakeVector` (`KismetMathLibrary.RandomFloatInRange` -250.0 250.0) (`KismetMathLibrary.RandomFloatInRange` -250.0 250.0)))))
  (if (`|EnumEquality` (`self.Faction`) (enumliteral `EFaction` "Alien"))
    (bind _returnvalue_2 (`|SpawnActorFromClass` "/Game/Blueprints/Units/BP_Unit_A_Transporter.BP_Unit_A_Transporter_C" _returnvalue "AdjustIfPossibleButAlwaysSpawn" "MultiplyWithRoot" null null))
    (`self.SetupSpawnedUnit` _returnvalue_2)
    (cast `/Game/Blueprints/Buildings/BP_Building_Mine` self
      (:`then`
        (`KismetArrayLibrary.Array_AddUnique` (`/Game/Blueprints/Units/BP_Unit_H_Transporter.Route` _returnvalue_2) self))
      (:`CastFailed`
        _))
    (`/Game/Blueprints/Units/BP_Unit_H_Transporter.StartRoute` _returnvalue_2)
    (else
      (bind _returnvalue_3 (`|SpawnActorFromClass` "/Game/Blueprints/Units/BP_Unit_H_Transporter.BP_Unit_H_Transporter_C" _returnvalue "AdjustIfPossibleButAlwaysSpawn" "MultiplyWithRoot" null null))
      (`self.SetupSpawnedUnit` _returnvalue_3)
      (cast `/Game/Blueprints/Buildings/BP_Building_Mine` self
        (:`then`
          (`KismetArrayLibrary.Array_AddUnique` (`/Game/Blueprints/Units/BP_Unit_H_Transporter.Route` _returnvalue_3) self))
        (:`CastFailed`
          _))
      (`/Game/Blueprints/Units/BP_Unit_H_Transporter.StartRoute` _returnvalue_3))))

(fn `AddBuildProgress`
  (params (Seconds :type "Float (double-precision)"))
  (bind _bdone (`self.IsConstructed`))
  (if (not _bdone)
    (set `self.BuildProgress` (+ (`self.BuildProgress`) (/ Seconds (`KismetMathLibrary.FMax` (`/Game/Blueprints/Data/PDA_Building.BuildTime` (`self.Data`)) 1.0))))
    (if (>= (`self.BuildProgress`) 1.0)
      (set `self.BuildProgress` 1.0)
      (set `self.bConstructed` true))
    (`self.RefreshBuildVisual`)))

(fn `ApplyTeamMaterial`)

(fn `BecomeGhost`
  (`self.SetGhost` self true)
  (set `self.bConstructed` false)
  (`self.SetActorEnableCollision` self false))

(fn `FinishTrain`
  (bind _output (`|GetArrayItem` (`self.ProductionQueue`)))
  (bind _cost (`/Game/Blueprints/Data/PDA_Unit.Cost` (`|GetArrayItem` (`/Game/Blueprints/Data/PDA_Building.Producible` (`self.Data`)) _output)))
  (if (not (`KismetArrayLibrary.Array_IsEmpty` (`self.ProductionQueue`)))
    (bind _asgm_default (cast `/Game/Blueprints/GM_Default` (`GameplayStatics.GetGameMode`)))
    (bind _state (`/Game/Blueprints/GM_Default.GetFactionState` _asgm_default (`self.Faction`)))
    (bind _keys (`BlueprintMapLibrary.Map_Keys` _cost))
    (for _array_element _keys
      (`/Game/Blueprints/Core/BP_FactionState.AddResource` _state _array_element (`BlueprintMapLibrary.Map_Find` _cost _array_element)))
    (set `self.bBypassQueue` true)
    (`self.TrainUnit` _output)
    (set `self.bBypassQueue` false)
    (`KismetArrayLibrary.Array_Remove` (`self.ProductionQueue`))
    (if (`KismetArrayLibrary.Array_IsNotEmpty` (`self.ProductionQueue`))
      (`KismetSystemLibrary.K2_SetTimer` self "FinishTrain" (`self.ProductionTime`)))))

(fn `GetHPPercent`
  (returns (Percent :type "Float (double-precision)"))
  (bind _maxhp (`self.GetMaxHP`))
  (return (`KismetMathLibrary.FClamp` (- 1.0 (/ (`self.DamageTaken`) _maxhp)))))

(fn `GetMaxHP`
  (returns (MaxHP :type "Float (double-precision)"))
  (return (`KismetMathLibrary.FMax` (`/Game/Blueprints/Data/PDA_Building.MaxHealth` (`self.Data`)) 1.0)))

(fn `GetSelectableDisplayName`
  (returns (Name :type Text))
  (return ""))

(fn `GetSelectableType`
  (returns (Type :type "/Game/Blueprints/E_SelectableType Enum"))
  (return "NewEnumerator2"))

(fn `IsConstructed`
  (returns (bDone :type Boolean))
  (return (`self.bConstructed`)))

(fn `QueueUnit`
  (params (Index :type Integer))
  (returns (Success :type Boolean))
  (bind _producible (`/Game/Blueprints/Data/PDA_Building.Producible` (`self.Data`)))
  (bind _cost (`/Game/Blueprints/Data/PDA_Unit.Cost` (`|GetArrayItem` _producible Index)))
  (bind _bdone (`self.IsConstructed`))
  (if (not _bdone)
    (return false)
    (elif (>= (`KismetArrayLibrary.Array_Length` (`self.ProductionQueue`)) 5)
      (`KismetSystemLibrary.PrintString` "File de production pleine (5 max)")
      (return false)
      (elif (not (`KismetArrayLibrary.Array_IsValidIndex` _producible Index))
        (return false)
        (else
          (bind _asgm_default (cast `/Game/Blueprints/GM_Default` (`GameplayStatics.GetGameMode`))
            (:`then`
              (bind _state (`/Game/Blueprints/GM_Default.GetFactionState` _asgm_default (`self.Faction`)))
              (bind _bcanafford (`/Game/Blueprints/Core/BP_FactionState.CanAfford` _state _cost))
              (if (not _bcanafford)
                (return false)
                (else
                  (`/Game/Blueprints/Core/BP_FactionState.Spend` _state _cost)
                  (`KismetArrayLibrary.Array_Add` (`self.ProductionQueue`) Index)
                  (`KismetSystemLibrary.PrintString` (`KismetStringLibrary.Concat_StrStr` "Production lancee. En file : " (`KismetStringLibrary.Conv_IntToString` (`KismetArrayLibrary.Array_Length` (`self.ProductionQueue`)))))
                  (if (== (`KismetArrayLibrary.Array_Length` (`self.ProductionQueue`)) 1)
                    (`KismetSystemLibrary.K2_SetTimer` self "FinishTrain" (`self.ProductionTime`)))
                  (return true))))
            (:`CastFailed`
              (return false))))))))

(fn `RefreshBuildVisual`
  (`self.SetActorScale3D` self (`KismetMathLibrary.MakeVector` 1.0 1.0 (+ 0.15 (* 0.85 (`KismetMathLibrary.FClamp` (`self.BuildProgress`)))))))

(fn `SetAllMaterials`
  (params (Material :type "MaterialInterface Object Reference"))
  (for _array_element (`self.K2_GetComponentsByClass` self "/Script/Engine.MeshComponent")
    (if (not (`KismetStringLibrary.Contains` (`KismetSystemLibrary.GetObjectName` _array_element) "Selection"))
      (for _index (range (+ (- (`PrimitiveComponent.GetNumMaterials` _array_element) 1) 1))
        (`PrimitiveComponent.SetMaterial` _array_element _index Material)))))

(fn `SetupSpawnedUnit`
  (params (Unit :type "/Game/Blueprints/Units/BP_UnitBase Object Reference"))
  (set `/Game/Blueprints/Units/BP_UnitBase.Faction` (`self.Faction`) Unit)
  (`/Game/Blueprints/Units/BP_UnitBase.ApplyFactionSkin` Unit)
  (`/Game/Blueprints/Units/BP_UnitBase.ApplyTeamMaterial` Unit)
  (if (`/Game/Blueprints/Data/PDA_Unit.bCanHarvest` (`/Game/Blueprints/Units/BP_UnitBase.Data` Unit))
    _))

(fn `Spawn Unit`
  (`|SpawnActorFromClass` "/Game/Blueprints/Units/BP_Unit_H_Worker.BP_Unit_H_Worker_C" (`SceneComponent.K2_GetComponentToWorld` (`self.Selection`)) "Undefined" "MultiplyWithRoot" null null))

(fn `StartConstruction`
  (`self.SetGhost` self false)
  (set `self.bConstructed` false)
  (set `self.BuildProgress` 0.0)
  (`self.SetActorEnableCollision` self true)
  (`self.RefreshBuildVisual`))

(fn `TakeHit`
  (params (Amount :type "Float (double-precision)") (Attacker :type "Actor Object Reference"))
  (set `self.DamageTaken` (+ (`self.DamageTaken`) Amount))
  (bind _maxhp (`self.GetMaxHP`))
  (if (>= (`self.DamageTaken`) _maxhp)
    (if (`/Game/Blueprints/Data/PDA_Building.bIsDepot` (`self.Data`))
      (if (`|EnumEquality` (`self.Faction`) (enumliteral `EFaction` "Human"))
        (`KismetSystemLibrary.PrintString` "DEFAITE : votre Hub a ete detruit" true true (struct :`R` 1 :`G` 0.2 :`B` 0.1 :`A` 1) 60.0)
        (else
          (`KismetSystemLibrary.PrintString` "VICTOIRE : le Hub alien est detruit" true true (struct :`R` 0.2 :`G` 1 :`B` 0.3 :`A` 1) 60.0))))
    (`self.K2_DestroyActor` self)))

(fn `TrainUnit`
  (params (Index :type Integer))
  (returns (bSuccess :type Boolean))
  (bind _returnvalue (`|EnumEquality` (`self.Faction`) (enumliteral `EFaction` "Alien")))
  (bind _producible (`/Game/Blueprints/Data/PDA_Building.Producible` (`self.Data`)))
  (bind _output (`|GetArrayItem` _producible Index))
  (bind _returnvalue_2 (`KismetMathLibrary.MakeTransform` (+ (`SceneComponent.K2_GetComponentLocation` (`self.SpawnPoint`)) (`KismetMathLibrary.MakeVector` (`KismetMathLibrary.RandomFloatInRange` -250.0 250.0) (`KismetMathLibrary.RandomFloatInRange` -250.0 250.0))) (`KismetMathLibrary.MakeRotator` 0.0)))
  (bind _cost (`/Game/Blueprints/Data/PDA_Unit.Cost` _output))
  (if (`self.bBypassQueue`)
    (bind _bdone (`self.IsConstructed`))
    (if (not _bdone)
      (return false)
      (else
        (bind _asgm_default (cast `/Game/Blueprints/GM_Default` (`GameplayStatics.GetGameMode`))
          (:`then`
            (bind _state (`/Game/Blueprints/GM_Default.GetFactionState` _asgm_default (`self.Faction`)))
            (if (< Index (`KismetArrayLibrary.Array_Length` _producible))
              (bind _bcanafford (`/Game/Blueprints/Core/BP_FactionState.CanAfford` _state _cost))
              (if _bcanafford
                (`/Game/Blueprints/Core/BP_FactionState.Spend` _state _cost)
                (if (== _output "/Game/Blueprints/Data/Units/DA_Unit_Transporter.DA_Unit_Transporter")
                  (`self.SpawnTransporter`)
                  (elif (== _output "/Game/Blueprints/Data/Units/DA_Unit_Drone.DA_Unit_Drone")
                    (bind _returnvalue_3 (`|SpawnActorFromClass` "/Game/Blueprints/Units/BP_Unit_H_Drone.BP_Unit_H_Drone_C" _returnvalue_2 "AdjustIfPossibleButAlwaysSpawn" "MultiplyWithRoot" null null))
                    (`self.SetupSpawnedUnit` _returnvalue_3)
                    (elif (and (not (`/Game/Blueprints/Data/PDA_Unit.bCanHarvest` _output)) _returnvalue)
                      (bind _returnvalue_4 (`|SpawnActorFromClass` "/Game/Blueprints/Units/BP_Unit_A_Tank.BP_Unit_A_Tank_C" _returnvalue_2 "AdjustIfPossibleButAlwaysSpawn" "MultiplyWithRoot" null null))
                      (`self.SetupSpawnedUnit` _returnvalue_4)
                      (elif (not (`/Game/Blueprints/Data/PDA_Unit.bCanHarvest` _output))
                        (bind _returnvalue_5 (`|SpawnActorFromClass` "/Game/Blueprints/Units/BP_Unit_H_Tank.BP_Unit_H_Tank_C" _returnvalue_2 "AdjustIfPossibleButAlwaysSpawn" "MultiplyWithRoot" null null))
                        (`self.SetupSpawnedUnit` _returnvalue_5)
                        (return true)
                        (elif _returnvalue
                          (bind _returnvalue_6 (`|SpawnActorFromClass` "/Game/Blueprints/Units/BP_Unit_A_Worker.BP_Unit_A_Worker_C" _returnvalue_2 "AdjustIfPossibleButAlwaysSpawn" "MultiplyWithRoot" null null))
                          (`self.SetupSpawnedUnit` _returnvalue_6)
                          (return true)
                          (else
                            (bind _returnvalue_7 (`|SpawnActorFromClass` "/Game/Blueprints/Units/BP_Unit_H_Worker.BP_Unit_H_Worker_C" _returnvalue_2 "AdjustIfPossibleButAlwaysSpawn" "MultiplyWithRoot" null null))
                            (`self.SetupSpawnedUnit` _returnvalue_7)
                            (return true)))))))
                (return true)
                (else
                  (return false)))
              (else
                (return false))))
          (:`CastFailed`
            (return false)))))
    (else
      (bind _success (`self.QueueUnit` Index))
      (return _success))))

(fn `UserConstructionScript`)