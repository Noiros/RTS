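; BP_BaseResource is a base resource actor holding a Remaining amount that can be drawn down.
; Take subtracts the requested amount, capped at Remaining, destroys the actor on a depletion check and returns a capped amount.
; The depletion check and return value recompute from the already reduced Remaining, so they can differ from the amount actually subtracted.
; Event graph and construction script are empty.
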(fn `Take`
  (params (Requested :type Integer))
  (returns (Taken :type Integer))
  (bind _remaining (`self.Remaining`))
  (bind _returnvalue (select `bool` (< Requested _remaining) :`false` _remaining :`true` Requested))
  (set `self.Remaining` (- _remaining _returnvalue))
  (if (<= (- _remaining _returnvalue) 0)
    (`self.K2_DestroyActor` self))
  (return _returnvalue))

(fn `UserConstructionScript`)