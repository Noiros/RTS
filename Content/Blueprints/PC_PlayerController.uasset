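; RTS player controller that handles camera control, selection and unit orders through Enhanced Input.
; Zoom input adjusts BP_Player, while move input and per-tick edge scrolling pan the pawn relative to camera yaw.
; Left click selects by type through interface messages, and drag-box selection takes units from HudPlayer, which also receives the selection.
; Right click orders selected units to move or harvest; HarvestMode turns the next left click into a harvest order.
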(event `self.ReceiveBeginPlay`
  (bind _returnvalue (subsystem `EnhancedInputLocalPlayerSubsystem`))
  ;[0.05098 0.05098 0.05098] Add Mapping Context
  (`/Engine/EditorBlueprintResources/StandardMacros.IsValid` _returnvalue
    (:`Is Valid`
      (`EnhancedInputSubsystemInterface.AddMappingContext` _returnvalue "/Game/Blueprints/Input/IMC_Default.IMC_Default" 0 (struct))
      (bind _ashud_player (cast `/Game/Blueprints/Widget/HudPlayer` (`self.GetHUD`)))
      (set `self.HUD` _ashud_player))))

(event `EnhancedInput|/Game/Blueprints/Input/Actions/IA_Zoom`
  (params (ActionValue :type "Float (double-precision)") (ElapsedSeconds :type "Float (double-precision)") (TriggeredSeconds :type "Float (double-precision)") (InputAction :type "InputAction Object Reference" :default "/Game/Blueprints/Input/Actions/IA_Zoom.IA_Zoom"))
  (:`Triggered`
    (bind _asbp_player (cast `/Game/Blueprints/BP_Player` (`GameplayStatics.GetPlayerPawn` 0)))
    (`/Game/Blueprints/BP_Player.SetZoom` _asbp_player (+ (`/Game/Blueprints/BP_Player.Zoom` _asbp_player) (* ActionValue (`self.CamZoomSpeed`))))))

(event `self.ReceiveTick`
  (params (DeltaSeconds :type "Float (single-precision)"))
  (`self.EdgeScroll`))

(event `EnhancedInput|/Game/Blueprints/Input/Actions/IA_Move`
  (params (ActionValue :type "Vector2D Structure") (ElapsedSeconds :type "Float (double-precision)") (TriggeredSeconds :type "Float (double-precision)") (InputAction :type "InputAction Object Reference" :default "/Game/Blueprints/Input/Actions/IA_Move.IA_Move"))
  (:`Triggered`
    (`self.MoveCamera` ActionValue_X ActionValue_Y)))

(event `EnhancedInput|/Game/Blueprints/Input/Actions/IA_LeftClick`
  (params (ActionValue :type Boolean) (ElapsedSeconds :type "Float (double-precision)") (TriggeredSeconds :type "Float (double-precision)") (InputAction :type "InputAction Object Reference" :default "/Game/Blueprints/Input/Actions/IA_LeftClick.IA_LeftClick"))
  (bind (_bblockinghit _binitialoverlap _time _distance _location _impactpoint _normal _impactnormal _physmat _hitactor) (`GameplayStatics.BreakHitResult` (`self.GetHitResultUnderCursorByChannel` "TraceTypeQuery2")))
  (:`Started`
    (if (`self.HarvestMode`)
      (`self.HarvestUnderCursor`)
      (else
        ; Comment
        (`self.BeginBoxSelect`)
        (bind _type (message `/Game/Blueprints/BPI_Selectable.GetSelectableType` _hitactor))
        (if (`|EnumInequality` _type (`self.SelectionMode`))
          (`self.UnselectAll`)
          (bind _output_get (set `self.SelectionMode` _type)))
        (switch `/Game/Blueprints/E_SelectableType` _output_get
          (:`NewEnumerator0`
            (`/Game/Blueprints/Widget/HudPlayer.SelectObject` :`self` (`self.HUD`)))
          (:`NewEnumerator1`
            (if (not (`|GetInputActionValue`))
              (`self.UnselectAll`))
            (`KismetArrayLibrary.Array_AddUnique` (`self.SelectedActors`) _hitactor)
            (message `/Game/Blueprints/BPI_Selectable.Select` _hitactor true)
            (`/Game/Blueprints/Widget/HudPlayer.SelectObject` (`self.HUD`) (`self.SelectedActors`)))
          (:`NewEnumerator2`
            (`KismetArrayLibrary.Array_AddUnique` (`self.SelectedActors`) _hitactor)
            (message `/Game/Blueprints/BPI_Selectable.Select` _hitactor true)
            (`/Game/Blueprints/Widget/HudPlayer.SelectObject` (`self.HUD`) (`self.SelectedActors`)))))))
  (:`Completed`
    (`self.EndBoxSelect`)))

(event `EnhancedInput|/Game/Blueprints/Input/Actions/IA_RightClick`
  (params (ActionValue :type Boolean) (ElapsedSeconds :type "Float (double-precision)") (TriggeredSeconds :type "Float (double-precision)") (InputAction :type "InputAction Object Reference" :default "/Game/Blueprints/Input/Actions/IA_RightClick.IA_RightClick"))
  (:`Started`
    (`self.IssueOrderUnderCursor`)))

(fn `BeginBoxSelect`
  (bind (_hit _location) (`self.GetLocationUnderCursor`))
  (bind _hud (`self.HUD`))
  (if _hit
    (set `/Game/Blueprints/Widget/HudPlayer.BoxStartWorld` _location _hud)
    (set `/Game/Blueprints/Widget/HudPlayer.bBoxSelecting` true _hud)))

(fn `EdgeScroll`
  (bind (_locationx _locationy _returnvalue) (`self.GetMousePosition`))
  (bind _screenmargin (`self.ScreenMargin`))
  (bind (_x _y) (`KismetMathLibrary.BreakVector2D` (`WidgetLayoutLibrary.GetViewportSize`)))
  (bind _returnvalue_2 (/ _locationx _x))
  (bind _returnvalue_3 (/ _locationy _y))
  (if (and _returnvalue (> _x 0.0))
    (`self.MoveCamera` (select `bool` (< _returnvalue_3 _screenmargin) :`false` (select `bool` (> _returnvalue_3 (- 1.0 _screenmargin)) :`false` 0.0 :`true` -1.0) :`true` 1.0) (select `bool` (< _returnvalue_2 _screenmargin) :`false` (select `bool` (> _returnvalue_2 (- 1.0 _screenmargin)) :`false` 0.0 :`true` 1.0) :`true` -1.0))))

(fn `EndBoxSelect`
  (bind (_locationx _locationy) (`self.GetMousePosition`))
  (bind _returnvalue (enumliteral `/Game/Blueprints/E_SelectableType` "NewEnumerator1"))
  (bind _hud (`self.HUD`))
  (bind _selectedactors (`self.SelectedActors`))
  (if (`/Game/Blueprints/Widget/HudPlayer.bBoxSelecting` _hud)
    (set `/Game/Blueprints/Widget/HudPlayer.bBoxSelecting` false _hud)
    (if (> (`KismetMathLibrary.Distance2D` (`KismetMathLibrary.MakeVector2D` _locationx _locationy) (`/Game/Blueprints/Widget/HudPlayer.BoxStart` _hud)) 8.0)
      (if (or (not (`|GetInputActionValue`)) (`|EnumInequality` (`self.SelectionMode`) _returnvalue))
        (`self.UnselectAll`))
      (set `self.SelectionMode` _returnvalue)
      (for _array_element (`/Game/Blueprints/Widget/HudPlayer.BoxUnits` _hud)
        (`KismetArrayLibrary.Array_AddUnique` _selectedactors _array_element)
        (message `/Game/Blueprints/BPI_Selectable.Select` _array_element true))
      (`/Game/Blueprints/Widget/HudPlayer.SelectObject` _hud _selectedactors))))

(fn `Follow`
  (params (Location :type "Vector Structure"))
  (bind _returnvalue (`self.K2_GetPawn`))
  (`Pawn.AddMovementInput` _returnvalue (`KismetMathLibrary.GetDirectionUnitVector` (`self.K2_GetActorLocation` _returnvalue) Location) 1.0 false))

(fn `GetLocationUnderCursor`
  (returns (Hit :type Boolean) (Location :type "Vector Structure"))
  (bind (_bblockinghit _binitialoverlap _time _distance _location) (`GameplayStatics.BreakHitResult` (`self.GetHitResultUnderCursorByChannel` "TraceTypeQuery1")))
  (return _bblockinghit _location))

(fn `GetLocationUnderFinger`
  (returns (Hit :type Boolean) (Location :type "Vector Structure"))
  (bind (_bblockinghit _binitialoverlap _time _distance _location) (`GameplayStatics.BreakHitResult` (`self.GetHitResultUnderFingerByChannel` "Touch1" "TraceTypeQuery1" false)))
  (return _bblockinghit _location))

(fn `HarvestUnderCursor`
  (set `self.HarvestMode` false)
  (bind _asbp_base_resource (cast `/Game/Blueprints/Resources/BP_BaseResource` (`.HitActor` (`GameplayStatics.BreakHitResult` (`self.GetHitResultUnderCursorByChannel` "TraceTypeQuery1" false)))))
  (for _array_element (`self.SelectedActors`)
    (bind _asbp_unit_base (cast `/Game/Blueprints/Units/BP_UnitBase` _array_element))
    (`/Game/Blueprints/Units/BP_UnitBase.OrderHarvest` _asbp_unit_base _asbp_base_resource)))

(fn `IssueOrderUnderCursor`
  (bind (_hitresult _returnvalue) (`self.GetHitResultUnderCursorByChannel` "TraceTypeQuery1" false))
  (bind (_bblockinghit _binitialoverlap _time _distance _location _impactpoint _normal _impactnormal _physmat _hitactor) (`GameplayStatics.BreakHitResult` _hitresult))
  (if _returnvalue
    (for _array_element (`self.SelectedActors`)
      (bind _asbp_unit_base (cast `/Game/Blueprints/Units/BP_UnitBase` _array_element))
      (bind _asbp_base_resource (cast `/Game/Blueprints/Resources/BP_BaseResource` _hitactor)
        (:`then`
          (`/Game/Blueprints/Units/BP_UnitBase.OrderHarvest` _asbp_unit_base _asbp_base_resource))
        (:`CastFailed`
          (`/Game/Blueprints/Units/BP_UnitBase.OrderMove` _asbp_unit_base _location))))))

(fn `MoveCamera`
  (params (Forward :type "Float (double-precision)") (Right :type "Float (double-precision)"))
  (bind (_x _y) (`KismetMathLibrary.GetAxes` (`KismetMathLibrary.MakeRotator` 0.0 0.0 (.yaw (`PlayerCameraManager.GetCameraRotation` (`GameplayStatics.GetPlayerCameraManager` 0))))))
  (`self.K2_AddActorWorldOffset` (`GameplayStatics.GetPlayerPawn` 0) (* (* (+ (* _x Forward) (* _y Right)) (`self.EdgeScrollSpeed`)) (`GameplayStatics.GetWorldDeltaSeconds`)) false false))

(fn `MoveTo`
  (params (Location :type "Vector Structure"))
  (`AIBlueprintHelperLibrary.SimpleMoveToLocation` self Location)
  (`NiagaraFunctionLibrary.SpawnSystemAtLocation` (`self.FXCursor`) Location))

(fn `UnselectAll`
  (bind _selectedactors (`self.SelectedActors`))
  (for _array_element _selectedactors
    (message `/Game/Blueprints/BPI_Selectable.Select` _array_element false))
  (`KismetArrayLibrary.Array_Clear` _selectedactors)
  (return))

(fn `UserConstructionScript`)