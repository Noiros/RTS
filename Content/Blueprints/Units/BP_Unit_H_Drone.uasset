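; Scout drone unit that can auto-explore the fog of war and takes its walk speed from its Data.
; A looping timer sends it to the nearest unexplored point from BP_FogOfWarManager, projected onto the navmesh, whenever the blackboard OrderType is zero.
; It picks a new target on arrival or timeout, first marking timed-out targets in the fog so unreachable spots are not retried.
; SetAutoExplore toggles the behavior, halting movement when disabled.
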(event `self.ReceiveBeginPlay`
  (bind _data (`self.Data`))
  (bind _speed (`/Game/Blueprints/Data/PDA_Unit.Speed` _data))
  (`KismetSystemLibrary.K2_SetTimer` self "ExploreTick" 0.5 true)
  (`/Engine/EditorBlueprintResources/StandardMacros.IsValid` _data
    (:`Is Valid`
      (if (> _speed 0.0)
        (set `CharacterMovementComponent.MaxWalkSpeed` _speed (`self.CharacterMovement`))))))

(event `ExploreTick`
  (bind _exploretarget (`self.ExploreTarget`))
  (bind _returnvalue (`self.K2_GetActorLocation` self))
  (bind _returnvalue_2 (+ (`self.ExploreElapsed`) 0.5))
  (bind _returnvalue_3 (`AIBlueprintHelperLibrary.GetBlackboard` (`self.GetController` self)))
  (if (`self.bAutoExplore`)
    (`/Engine/EditorBlueprintResources/StandardMacros.IsValid` _returnvalue_3
      (:`Is Valid`
        (if (!= (`BlackboardComponent.GetValueAsEnum` _returnvalue_3 "OrderType") 0)
          (set `self.bHasExploreTarget` false)
          (else
            (bind _asbp_fog_of_war_manager (cast `/Game/Blueprints/Core/BP_FogOfWarManager` (`ActorScanner.GetFirstCachedActorOfClass` "/Game/Blueprints/Core/BP_FogOfWarManager.BP_FogOfWarManager_C")))
            (bind _bhuman (`self.IsHuman`))
            (if (`self.bHasExploreTarget`)
              (set `self.ExploreElapsed` _returnvalue_2)
              (if (<= (`KismetMathLibrary.Vector_Distance2D` _returnvalue _exploretarget) 450.0)
                (set `self.bHasExploreTarget` false)
                (elif (>= _returnvalue_2 15.0)
                  (`/Game/Blueprints/Core/BP_FogOfWarManager.MarkSource` _asbp_fog_of_war_manager _exploretarget 1200.0 _bhuman)
                  (set `self.bHasExploreTarget` false))))
            (if (not (`self.bHasExploreTarget`))
              (bind _location (`/Game/Blueprints/Core/BP_FogOfWarManager.GetNearestUnexplored` _asbp_fog_of_war_manager _bhuman _returnvalue))
              (if (> (`KismetMathLibrary.Vector_Distance2D` _location _returnvalue) 200.0)
                (bind (_projectedlocation _returnvalue_4) (`NavigationSystemV1.K2_ProjectPointToNavigation` _location null null (`KismetMathLibrary.MakeVector` 600.0 600.0 1000.0)))
                (bind _returnvalue_5 (select `bool` _returnvalue_4 :`false` _location :`true` _projectedlocation))
                (set `self.ExploreTarget` _returnvalue_5)
                (set `self.ExploreElapsed` 0.0)
                (set `self.bHasExploreTarget` true)
                (`AIController.MoveToLocation` (`AIBlueprintHelperLibrary.GetAIController` self) _returnvalue_5 100.0 true true true true null true)))))))))

(fn `GetSelectableDisplayName`
  (returns (Name :type Text))
  (return "Drone éclaireur"))

(fn `SetAutoExplore`
  (params (bEnable :type Boolean))
  (set `self.bAutoExplore` bEnable)
  (set `self.bHasExploreTarget` false)
  (if (not bEnable)
    (`Controller.StopMovement` (`AIBlueprintHelperLibrary.GetAIController` self))))

(fn `UserConstructionScript`
  (`parent.UserConstructionScript`))