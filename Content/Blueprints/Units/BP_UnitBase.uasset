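; Base RTS unit for Human and Alien factions, driven by a data asset for stats, abilities and meshes.
; Order functions write move, harvest, build and attack orders to the AI controller's Blackboard, falling back to moving when incapable.
; Throttled Tick checks chase and damage targets, scan for enemies during attack-move, and advance construction on build targets.
; Hits accumulate damage until destruction; idle or attacking armed units without a unit target retaliate.
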(event `self.ReceiveTick`
  (params (DeltaSeconds :type "Float (single-precision)"))
  (`self.CombatTick`)
  (`self.WorkTick`))

(event `/Game/Blueprints/BPI_Selectable.Select`
  (params (Selected :type Boolean))
  (`SceneComponent.SetVisibility` (`self.Selection`) Selected true))

(event `self.ReceiveBeginPlay`
  (`KismetSystemLibrary.Delay` 1.0)
  (if (`self.bHarvestOnStart`)
    _))

(event `/Game/Blueprints/BPI_Unit.MoveTo`
  (params (TargetPos :type "Vector Structure"))
  (`BlackboardComponent.SetValueAsVector` (`AIBlueprintHelperLibrary.GetBlackboard` (`self.GetController`)) "Target" TargetPos))

(fn `AcquireTarget`
  (params (Radius :type "Float (double-precision)"))
  (bind _enemy (`self.FindNearestEnemy` Radius))
  (set `self.AttackTarget` _enemy)
  (`/Engine/EditorBlueprintResources/StandardMacros.IsValid` _enemy
    (:`Is Valid`
      (if (`self.bAttackMove`)
        (`BlackboardComponent.SetValueAsEnum` (`AIBlueprintHelperLibrary.GetBlackboard` (`self.GetController`)) "OrderType" 4)))))

(fn `ApplyFactionSkin`
  (bind _data (`self.Data`))
  (bind _alienstaticmesh (`/Game/Blueprints/Data/PDA_Unit.AlienStaticMesh` _data))
  (bind _alienskeletalmesh (`/Game/Blueprints/Data/PDA_Unit.AlienSkeletalMesh` _data))
  (if (`|EnumEquality` (`self.Faction`) (enumliteral `EFaction` "Alien"))
    (`/Engine/EditorBlueprintResources/StandardMacros.IsValid` _data
      (:`Is Valid`
        (`|ExecutionSequence`
          (:`then_0`
            (`/Engine/EditorBlueprintResources/StandardMacros.IsValid` _alienstaticmesh
              (:`Is Valid`
                (`StaticMeshComponent.SetStaticMesh` (`self.TMP`) _alienstaticmesh))))
          (:`then_1`
            (`/Engine/EditorBlueprintResources/StandardMacros.IsValid` _alienskeletalmesh
              (:`Is Valid`
                (`SkeletalMeshComponent.SetSkeletalMeshAsset` (`self.Mesh`) _alienskeletalmesh)))))))))

(fn `ApplyTeamMaterial`)

(fn `CombatTick`
  (bind _returnvalue (`KismetSystemLibrary.GetGameTimeInSeconds`))
  (bind _data (`self.Data`))
  (bind _battackmove (`self.bAttackMove`))
  (bind _returnvalue_2 (`AIBlueprintHelperLibrary.GetBlackboard` (`self.GetController`)))
  (bind _returnvalue_3 (`BlackboardComponent.GetValueAsEnum` _returnvalue_2 "OrderType"))
  (if (and (> (`/Game/Blueprints/Data/PDA_Unit.AttackDamage` _data) 0.0) (>= (- _returnvalue (`self.LastCombatCheck`)) 0.25))
    (set `self.LastCombatCheck` _returnvalue)
    (`/Engine/EditorBlueprintResources/StandardMacros.IsValid` (`self.AttackTarget`)
      (:`Is Valid`
        (`self.EngageTarget`))
      (:`Is Not Valid`
        (if (== _returnvalue_3 4)
          (`Controller.StopMovement` (`AIBlueprintHelperLibrary.GetAIController` self))
          (if _battackmove
            (`self.ResumeAttackMove`)
            (else
              (`BlackboardComponent.SetValueAsEnum` _returnvalue_2 "OrderType" 0)))
          (elif (== _returnvalue_3 0)
            (set `self.bAttackMove` false)
            (elif (and (== _returnvalue_3 1) _battackmove)
              (`self.AcquireTarget` (`/Game/Blueprints/Data/PDA_Unit.VisionRadius` _data)))))))))

(fn `DealDamage`
  (params (Target :type "Actor Object Reference") (Amount :type "Float (double-precision)"))
  (bind _asbp_unit_base (cast `/Game/Blueprints/Units/BP_UnitBase` Target)
    (:`then`
      (`self.TakeHit` _asbp_unit_base Amount self))
    (:`CastFailed`
      (bind _asbp_base_building (cast `/Game/Blueprints/Buildings/BP_BaseBuilding` Target))
      (`/Game/Blueprints/Buildings/BP_BaseBuilding.TakeHit` _asbp_base_building Amount self))))

(fn `EngageTarget`
  (bind _returnvalue (`KismetSystemLibrary.GetGameTimeInSeconds`))
  (bind _attacktarget (`self.AttackTarget`))
  (bind _data (`self.Data`))
  (bind _returnvalue_2 (`AIBlueprintHelperLibrary.GetAIController` self))
  (bind (_origin _boxextent) (`self.GetActorBounds` _attacktarget true false))
  (bind _attackrange (`/Game/Blueprints/Data/PDA_Unit.AttackRange` _data))
  (bind _returnvalue_3 (`KismetMathLibrary.FMax` (.x _boxextent) (.y _boxextent)))
  (if (<= (- (`self.GetDistanceTo` self _attacktarget) _returnvalue_3) _attackrange)
    (`Controller.StopMovement` _returnvalue_2)
    (`self.K2_SetActorRotation` self (`KismetMathLibrary.MakeRotator` 0.0 0.0 (.yaw (`KismetMathLibrary.FindLookAtRotation` (`self.K2_GetActorLocation` self) (`self.K2_GetActorLocation` _attacktarget)))) false)
    (if (>= (- _returnvalue (`self.LastAttackTime`)) (`/Game/Blueprints/Data/PDA_Unit.AttackCooldown` _data))
      (set `self.LastAttackTime` _returnvalue)
      (`self.DealDamage` _attacktarget (`/Game/Blueprints/Data/PDA_Unit.AttackDamage` _data)))
    (else
      (`AIController.MoveToActor` _returnvalue_2 _attacktarget (+ _returnvalue_3 (* _attackrange 0.7)) true true true null true))))

(fn `FindNearestEnemy`
  (params (Radius :type "Float (double-precision)"))
  (returns (Enemy :type "Actor Object Reference"))
  (set `self.ScanBest` null)
  (set `self.ScanBestDist` Radius)
  (bind _outactors (`GameplayStatics.GetAllActorsOfClass` "BP_UnitBase_C"))
  (for _array_element _outactors
    (bind _benemy (`self.IsEnemy` _array_element))
    (if _benemy
      (bind _returnvalue (`self.GetDistanceTo` self _array_element))
      (if (< _returnvalue (`self.ScanBestDist`))
        (set `self.ScanBestDist` _returnvalue)
        (set `self.ScanBest` _array_element))))
  (`/Engine/EditorBlueprintResources/StandardMacros.IsValid` (`self.ScanBest`)
    (:`Is Valid`
      (return (`self.ScanBest`)))
    (:`Is Not Valid`
      (bind _outactors_2 (`GameplayStatics.GetAllActorsOfClass` "/Game/Blueprints/Buildings/BP_BaseBuilding.BP_BaseBuilding_C"))
      (for _array_element_2 _outactors_2
        (bind _benemy_2 (`self.IsEnemy` _array_element_2))
        (if _benemy_2
          (bind (_origin _boxextent) (`self.GetActorBounds` _array_element_2 true false))
          (bind _returnvalue_2 (- (`self.GetDistanceTo` self _array_element_2) (`KismetMathLibrary.FMax` (.x _boxextent) (.y _boxextent))))
          (if (< _returnvalue_2 (`self.ScanBestDist`))
            (set `self.ScanBestDist` _returnvalue_2)
            (set `self.ScanBest` _array_element_2))))
      (return (`self.ScanBest`)))))

(fn `FindNearestResource`
  (locals (BestNode :type "/Game/Blueprints/Resources/BP_BaseResource Object Reference") (BestDistance :type "Float (double-precision)"))
  (bind _returnvalue (`AIBlueprintHelperLibrary.GetBlackboard` (`self.GetController`)))
  (set `local.BestDistance` 100000000.0)
  (set `local.BestNode` null)
  (bind _outactors (`GameplayStatics.GetAllActorsOfClass` "/Game/Blueprints/Resources/BP_BaseResource.BP_BaseResource_C"))
  (for _array_element _outactors
    (if (and (and (`|EnumEquality` (`/Game/Blueprints/Resources/BP_BaseResource.ResourceType` _array_element) (`self.CarriedResource`)) (> (`/Game/Blueprints/Resources/BP_BaseResource.Remaining` _array_element) 0)) (not (`self.ActorHasTag` _array_element "Deposit")))
      (bind _returnvalue_2 (`self.GetDistanceTo` self _array_element))
      (if (< _returnvalue_2 (`local.BestDistance`))
        (set `local.BestDistance` _returnvalue_2)
        (set `local.BestNode` _array_element))))
  (`/Engine/EditorBlueprintResources/StandardMacros.IsValid` (`local.BestNode`)
    (:`Is Valid`
      (`BlackboardComponent.SetValueAsObject` _returnvalue "TargetActor" (`local.BestNode`)))
    (:`Is Not Valid`
      (`BlackboardComponent.SetValueAsEnum` _returnvalue "OrderType" 0))))

(fn `GetHPPercent`
  (returns (Percent :type "Float (double-precision)"))
  (bind _maxhp (`self.GetMaxHP`))
  (return (`KismetMathLibrary.FClamp` (- 1.0 (/ (`self.DamageTaken`) _maxhp)))))

(fn `GetMaxHP`
  (returns (MaxHP :type "Float (double-precision)"))
  (return (`KismetMathLibrary.FMax` (`/Game/Blueprints/Data/PDA_Unit.MaxHealth` (`self.Data`)) 1.0)))

(fn `GetSelectableDisplayName`
  (returns (Name :type Text))
  (return ""))

(fn `GetSelectableType`
  (returns (Type :type "/Game/Blueprints/E_SelectableType Enum"))
  (return "NewEnumerator1"))

(fn `IsEnemy`
  (params (Other :type "Actor Object Reference"))
  (returns (bEnemy :type Boolean))
  (bind _asbp_unit_base (cast `/Game/Blueprints/Units/BP_UnitBase` Other)
    (:`then`
      (bind _bhuman (`self.IsHuman` _asbp_unit_base))
      (bind _bhuman_2 (`self.IsHuman`))
      (return (!= _bhuman _bhuman_2)))
    (:`CastFailed`
      (bind _asbp_base_building (cast `/Game/Blueprints/Buildings/BP_BaseBuilding` Other)
        (:`then`
          (return (`|EnumInequality` (`/Game/Blueprints/Buildings/BP_BaseBuilding.Faction` _asbp_base_building) (`self.Faction`))))
        (:`CastFailed`
          (return false))))))

(fn `IsHuman`
  (returns (bHuman :type Boolean))
  (return (`|EnumEquality` (`self.Faction`) (enumliteral `EFaction` "Human"))))

(fn `OrderAttack`
  (params (Target :type "Actor Object Reference"))
  (if (> (`/Game/Blueprints/Data/PDA_Unit.AttackDamage` (`self.Data`)) 0.0)
    (set `self.BuildTarget` null)
    (set `self.bAttackMove` false)
    (set `self.AttackTarget` Target)
    (`BlackboardComponent.SetValueAsEnum` (`AIBlueprintHelperLibrary.GetBlackboard` (`self.GetController`)) "OrderType" 4)
    (else
      (`self.OrderMove` (`self.K2_GetActorLocation` Target)))))

(fn `OrderAttackMove`
  (params (Location :type "Vector Structure"))
  (`self.OrderMove` Location)
  (if (> (`/Game/Blueprints/Data/PDA_Unit.AttackDamage` (`self.Data`)) 0.0)
    (set `self.bAttackMove` true)
    (set `self.AttackMoveDest` Location)))

(fn `OrderBuild`
  (params (Building :type "/Game/Blueprints/Buildings/BP_BaseBuilding Object Reference"))
  (if (`/Game/Blueprints/Data/PDA_Unit.bCanHarvest` (`self.Data`))
    (set `self.AttackTarget` null)
    (set `self.bAttackMove` false)
    (set `self.BuildTarget` Building)
    (`BlackboardComponent.SetValueAsEnum` (`AIBlueprintHelperLibrary.GetBlackboard` (`self.GetController`)) "OrderType" 3)
    (else
      (`self.OrderMove` (`self.K2_GetActorLocation` Building)))))

(fn `OrderHarvest`
  (params (Resource :type "/Game/Blueprints/Resources/BP_BaseResource Object Reference"))
  (bind _returnvalue (`AIBlueprintHelperLibrary.GetBlackboard` (`self.GetController`)))
  (set `self.AttackTarget` null)
  (set `self.BuildTarget` null)
  (set `self.bAttackMove` false)
  (if (and (`/Game/Blueprints/Data/PDA_Unit.bCanHarvest` (`self.Data`)) (not (`self.ActorHasTag` Resource "Deposit")))
    (`BlackboardComponent.SetValueAsObject` _returnvalue "TargetActor" Resource)
    (`BlackboardComponent.SetValueAsEnum` _returnvalue "OrderType" 2)
    (else
      (`self.OrderMove` (`self.K2_GetActorLocation` Resource)))))

(fn `OrderMove`
  (params (Location :type "Vector Structure"))
  (bind _returnvalue (`AIBlueprintHelperLibrary.GetBlackboard` (`self.GetController`)))
  (set `self.AttackTarget` null)
  (set `self.BuildTarget` null)
  (set `self.bAttackMove` false)
  (`BlackboardComponent.SetValueAsEnum` _returnvalue "OrderType" 0)
  (`BlackboardComponent.SetValueAsVector` _returnvalue "Target" Location)
  (`BlackboardComponent.SetValueAsEnum` _returnvalue "OrderType" 1))

(fn `ResumeAttackMove`
  (`self.OrderAttackMove` (`self.AttackMoveDest`)))

(fn `SetAllMaterials`
  (params (Material :type "MaterialInterface Object Reference"))
  (for _array_element (`self.K2_GetComponentsByClass` self "/Script/Engine.MeshComponent")
    (if (not (`KismetStringLibrary.Contains` (`KismetSystemLibrary.GetObjectName` _array_element) "Selection"))
      (for _index (range (+ (- (`PrimitiveComponent.GetNumMaterials` _array_element) 1) 1))
        (`PrimitiveComponent.SetMaterial` _array_element _index Material)))))

(fn `StartHarvestNearest`
  (bind _returnvalue (`AIBlueprintHelperLibrary.GetBlackboard` (`self.GetController`)))
  (set `self.CarriedResource` (enumliteral `EResource` "Ore"))
  (`self.FindNearestResource`)
  (`/Engine/EditorBlueprintResources/StandardMacros.IsValid` (`BlackboardComponent.GetValueAsObject` _returnvalue "TargetActor")
    (:`Is Valid`
      (`BlackboardComponent.SetValueAsEnum` _returnvalue "OrderType" 2))))

(fn `TakeHit`
  (params (Amount :type "Float (double-precision)") (Attacker :type "Actor Object Reference"))
  (bind _returnvalue (`BlackboardComponent.GetValueAsEnum` (`AIBlueprintHelperLibrary.GetBlackboard` (`self.GetController`)) "OrderType"))
  (set `self.DamageTaken` (+ (`self.DamageTaken`) Amount))
  (bind _maxhp (`self.GetMaxHP`))
  (if (>= (`self.DamageTaken`) _maxhp)
    (`self.K2_DestroyActor` self)
    (else
      (cast `/Game/Blueprints/Units/BP_UnitBase` (`self.AttackTarget`)
        (:`CastFailed`
          (if (and (> (`/Game/Blueprints/Data/PDA_Unit.AttackDamage` (`self.Data`)) 0.0) (or (== _returnvalue 0) (== _returnvalue 4)))
            (set `self.AttackTarget` Attacker)))))))

(fn `UserConstructionScript`)

(fn `WorkTick`
  (bind _returnvalue (`KismetSystemLibrary.GetGameTimeInSeconds`))
  (bind _buildtarget (`self.BuildTarget`))
  (bind (_origin _boxextent) (`self.GetActorBounds` _buildtarget true false))
  (bind _returnvalue_2 (`KismetMathLibrary.FMax` (.x _boxextent) (.y _boxextent)))
  (if (>= (- _returnvalue (`self.LastWorkCheck`)) 0.25)
    (set `self.WorkDt` (`KismetMathLibrary.FMin` (- _returnvalue (`self.LastWorkCheck`)) 0.5))
    (set `self.LastWorkCheck` _returnvalue)
    (`/Engine/EditorBlueprintResources/StandardMacros.IsValid` _buildtarget
      (:`Is Valid`
        (bind _bdone (`/Game/Blueprints/Buildings/BP_BaseBuilding.IsConstructed` _buildtarget))
        (if _bdone
          (set `self.BuildTarget` null)
          (`self.OrderMove` (`self.K2_GetActorLocation`))
          (elif (<= (- (`self.GetDistanceTo` self _buildtarget) _returnvalue_2) 250.0)
            (`Controller.StopMovement` (`AIBlueprintHelperLibrary.GetAIController` self))
            (`/Game/Blueprints/Buildings/BP_BaseBuilding.AddBuildProgress` _buildtarget (`self.WorkDt`))
            (else
              (`AIController.MoveToActor` (`AIBlueprintHelperLibrary.GetAIController` self) _buildtarget (+ _returnvalue_2 150.0) true true true null true))))))))