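; GM_Default is the default game mode that sets up per-faction state for the human and alien factions.
; On BeginPlay it spawns a BP_FactionState actor for each faction data asset, copying in the faction, data and starting resources.
; Spawned states are stored in the FactionStates array, and GetFactionState looks one up by faction with a linear search.
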(event `self.ReceiveBeginPlay`
  (`self.CreateFactionState` (`self.HumanFactionData`))
  (`self.CreateFactionState` (`self.AlienFactionData`)))

(fn `CreateFactionState`
  (params (Data :type "/Game/Blueprints/Data/PDA_Faction Object Reference"))
  (bind _returnvalue (`|SpawnActorFromClass` "/Game/Blueprints/Core/BP_FactionState.BP_FactionState_C" (`KismetMathLibrary.MakeTransform` (0.0 0.0 0.0)) "Undefined" "MultiplyWithRoot" null null))
  (set `/Game/Blueprints/Core/BP_FactionState.Faction` (`/Game/Blueprints/Data/PDA_Faction.Faction` Data) _returnvalue)
  (set `/Game/Blueprints/Core/BP_FactionState.FactionData` Data _returnvalue)
  (set `/Game/Blueprints/Core/BP_FactionState.Resources` (`/Game/Blueprints/Data/PDA_Faction.StartingResources` Data) _returnvalue)
  (`KismetArrayLibrary.Array_Add` (`self.FactionStates`) _returnvalue))

(fn `GetFactionState`
  (params (Faction :type "EFaction Enum" :default "None"))
  (returns (State :type "/Game/Blueprints/Core/BP_FactionState Object Reference"))
  (for _array_element (`self.FactionStates`)
    (if (`|EnumEquality` (`/Game/Blueprints/Core/BP_FactionState.Faction` _array_element) Faction)
      (return _array_element)))
  (return null))

(fn `UserConstructionScript`)