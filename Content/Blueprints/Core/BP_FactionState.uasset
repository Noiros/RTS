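; BP_FactionState holds a faction's resource pool as a map of resource to amount and handles costs against it.
; GetResource reads the map, and AddResource writes the new total and fires OnResourcesChanged.
; CanAfford checks a cost map against the pool.
; Spend deducts only if CanAfford passes, using negative AddResource calls, so the change notification fires once per cost entry and no success result is returned.
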(fn `AddResource`
  (params (Resource :type "EResource Enum" :default "Ore") (Amount :type Integer))
  (`BlueprintMapLibrary.Map_Add` (`self.Resources`) Resource (+ (`BlueprintMapLibrary.Map_Find` (`self.Resources`) Resource) Amount))
  (`self.OnResourcesChanged`))

(fn `CanAfford`
  (params (Cost :type "Map of EResource Enum to Integer"))
  (returns (bCanAfford :type Boolean))
  (bind _keys (`BlueprintMapLibrary.Map_Keys` Cost))
  (for _array_element _keys
    (bind _amount (`self.GetResource` _array_element))
    (if (< _amount (`BlueprintMapLibrary.Map_Find` Cost _array_element))
      (return false)))
  (return true))

(fn `GetResource`
  (params (Resource :type "EResource Enum" :default "Ore"))
  (returns (Amount :type Integer))
  (return (`BlueprintMapLibrary.Map_Find` (`self.Resources`) Resource)))

(fn `Spend`
  (params (Cost :type "Map of EResource Enum to Integer"))
  (bind _bcanafford (`self.CanAfford` Cost))
  (if _bcanafford
    (bind _keys (`BlueprintMapLibrary.Map_Keys` Cost))
    (for _array_element _keys
      (`self.AddResource` _array_element (- 0 (`BlueprintMapLibrary.Map_Find` Cost _array_element))))))

(fn `UserConstructionScript`)