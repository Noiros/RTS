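; BP_Commander is the RTS AI opponent that runs the Alien faction's economy, army and attacks.
; A looping two-second timer runs Think, which rescans cached buildings and units for hubs, unit counts and humans near the Alien hub.
; It wakes idle harvesters via their blackboard order, then trains workers or soldiers, diverting soldiers to any threat.
; At wave size, it sends soldiers at the player's hub and enlarges the next wave.
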(event `self.ReceiveBeginPlay`
  (`KismetSystemLibrary.K2_SetTimer` self "Think" 2.0 true))

(fn `DefendIfThreat`
  (`/Engine/EditorBlueprintResources/StandardMacros.IsValid` (`self.Threat`)
    (:`Is Valid`
      (set `self.Phase` "Defense")
      (`self.SendSoldiers` (`self.Threat`)))))

(fn `ScanWorld`
  (set `self.Workers` 0)
  (set `self.Soldiers` 0)
  (set `self.Threat` null)
  (bind _outactors (`ActorScanner.GetCachedActorsOfClass` "/Game/Blueprints/Buildings/BP_BaseBuilding.BP_BaseBuilding_C"))
  (for _array_element _outactors
    (if (`/Game/Blueprints/Data/PDA_Building.bIsDepot` (`/Game/Blueprints/Buildings/BP_BaseBuilding.Data` _array_element))
      (if (`|EnumEquality` (`/Game/Blueprints/Buildings/BP_BaseBuilding.Faction` _array_element) (enumliteral `EFaction` "Alien"))
        (set `self.AlienHub` _array_element)
        (else
          (set `self.PlayerHub` _array_element)))))
  (bind _outactors_2 (`ActorScanner.GetCachedActorsOfClass` "/Game/Blueprints/Units/BP_UnitBase.BP_UnitBase_C"))
  (for _array_element_2 _outactors_2
    (if (`|EnumEquality` (`/Game/Blueprints/Units/BP_UnitBase.Faction` _array_element_2) "Human")
      (`/Engine/EditorBlueprintResources/StandardMacros.IsValid` (`self.AlienHub`)
        (:`Is Valid`
          (if (< (`self.GetDistanceTo` _array_element_2 (`self.AlienHub`)) (`self.DefenseRadius`))
            (set `self.Threat` _array_element_2))))
      (elif (`/Game/Blueprints/Data/PDA_Unit.bCanHarvest` (`/Game/Blueprints/Units/BP_UnitBase.Data` _array_element_2))
        (set `self.Workers` (+ (`self.Workers`) 1))
        (else
          (set `self.Soldiers` (+ (`self.Soldiers`) 1)))))))

(fn `SendSoldiers`
  (params (Target :type "Actor Object Reference"))
  (bind _outactors (`ActorScanner.GetCachedActorsOfClass` "/Game/Blueprints/Units/BP_UnitBase.BP_UnitBase_C"))
  (for _array_element _outactors
    (if (and (not (`|EnumEquality` (`/Game/Blueprints/Units/BP_UnitBase.Faction` _array_element) "Human")) (not (`/Game/Blueprints/Data/PDA_Unit.bCanHarvest` (`/Game/Blueprints/Units/BP_UnitBase.Data` _array_element))))
      (`/Game/Blueprints/Units/BP_UnitBase.OrderAttack` _array_element Target))))

(fn `Think`
  (`self.ScanWorld`)
  (`/Engine/EditorBlueprintResources/StandardMacros.IsValid` (`self.AlienHub`)
    (:`Is Valid`
      (`self.WakeIdleWorkers`)
      (if (< (`self.Workers`) (`self.TargetWorkers`))
        (set `self.Phase` "Developpement")
        (`/Game/Blueprints/Buildings/BP_BaseBuilding.TrainUnit` (`self.AlienHub`) 0)
        (`self.DefendIfThreat`)
        (elif (< (`self.Soldiers`) (`self.WaveSize`))
          (set `self.Phase` "Armee")
          (`/Game/Blueprints/Buildings/BP_BaseBuilding.TrainUnit` (`self.AlienHub`) 1)
          (`self.DefendIfThreat`)
          (else
            (`/Engine/EditorBlueprintResources/StandardMacros.IsValid` (`self.PlayerHub`)
              (:`Is Valid`
                (set `self.Phase` "Attaque")
                (`self.SendSoldiers` (`self.PlayerHub`))
                (set `self.WaveSize` (+ (`self.WaveSize`) 2))))))))))

(fn `UserConstructionScript`)

(fn `WakeIdleWorkers`
  (bind _outactors (`ActorScanner.GetCachedActorsOfClass` "/Game/Blueprints/Units/BP_UnitBase.BP_UnitBase_C"))
  (for _array_element _outactors
    (if (and (not (`|EnumEquality` (`/Game/Blueprints/Units/BP_UnitBase.Faction` _array_element) "Human")) (`/Game/Blueprints/Data/PDA_Unit.bCanHarvest` (`/Game/Blueprints/Units/BP_UnitBase.Data` _array_element)))
      (if (== (`BlackboardComponent.GetValueAsEnum` (`AIBlueprintHelperLibrary.GetBlackboard` _array_element) "OrderType") 0)
        (`/Game/Blueprints/Units/BP_UnitBase.StartHarvestNearest` _array_element)))))