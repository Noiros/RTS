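; Fog-of-war manager that tracks visible and explored cells for Human and Alien factions on a grid over the camera bounds.
; A looping timer stamps unit and building vision, then hides non-human units out of sight and non-human buildings in unexplored cells.
; Human vision is painted into render targets for a world-space fog plane material and the minimap, which also plots units and buildings.
; It also answers visibility and nearest-unexplored-cell queries.
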(event `self.ReceiveBeginPlay`
  (bind _returnvalue (`GameplayStatics.GetPlayerController` 0))
  (bind _aspc_player_controller (cast `/Game/Blueprints/PC_PlayerController` _returnvalue))
  (set `self.CellSize` 1000.0)
  (bind _camboundsmin (`/Game/Blueprints/PC_PlayerController.CamBoundsMin` _aspc_player_controller))
  (set `self.BoundsMin` _camboundsmin)
  (bind _camboundsmax (`/Game/Blueprints/PC_PlayerController.CamBoundsMax` _aspc_player_controller))
  (set `self.GridW` (+ (`KismetMathLibrary.FTrunc` (/ (- (.x _camboundsmax) (.x _camboundsmin)) 1000.0)) 1))
  (set `self.GridH` (+ (`KismetMathLibrary.FTrunc` (/ (- (.y _camboundsmax) (.y _camboundsmin)) 1000.0)) 1))
  (for _ (range (+ (- (* (`self.GridW`) (`self.GridH`)) 1) 1))
    (`KismetArrayLibrary.Array_Add` (`self.ExploredHuman`))
    (`KismetArrayLibrary.Array_Add` (`self.ExploredAlien`))
    (`KismetArrayLibrary.Array_Add` (`self.VisibleHuman`))
    (`KismetArrayLibrary.Array_Add` (`self.VisibleAlien`)))
  (bind _returnvalue_2 (`KismetRenderingLibrary.CreateRenderTarget2D` 64 64 "RTF_RGBA8" (make `LinearColor` 1.0 1.0 1.0 1.0)))
  (set `self.FogRT` _returnvalue_2)
  (bind _returnvalue_3 (`KismetRenderingLibrary.CreateRenderTarget2D` 128 128 "RTF_RGBA8" (make `LinearColor` 0.0 0.0 0.0 1.0)))
  (set `self.MiniRT` _returnvalue_3)
  (bind _returnvalue_4 (`|SpawnActorFromClass` "/Script/Engine.StaticMeshActor" (`KismetMathLibrary.MakeTransform` (`KismetMathLibrary.MakeVector` (+ (.x _camboundsmin) (* 0.5 (* (`self.GridW`) 1000.0))) (+ (.y _camboundsmin) (* 0.5 (* (`self.GridH`) 1000.0))) 2250.0) (struct) (`KismetMathLibrary.MakeVector` 640.0 640.0 1.0)) "AlwaysSpawn" "MultiplyWithRoot" null null))
  (bind _staticmeshcomponent (`StaticMeshActor.StaticMeshComponent` _returnvalue_4))
  (`SceneComponent.SetMobility` _staticmeshcomponent "Movable")
  (`PrimitiveComponent.SetCastShadow` _staticmeshcomponent false)
  (`StaticMeshComponent.SetStaticMesh` _staticmeshcomponent "/Engine/BasicShapes/Plane.Plane")
  (`PrimitiveComponent.SetCollisionEnabled` _staticmeshcomponent "NoCollision")
  (bind _returnvalue_5 (`PrimitiveComponent.CreateDynamicMaterialInstance` _staticmeshcomponent 0 "/Game/Materials/M_FogOfWar.M_FogOfWar" "None"))
  (`MaterialInstanceDynamic.SetTextureParameterValue` _returnvalue_5 "FogMask" (`self.FogRT`))
  (bind _returnvalue_6 (`|CreateWidget` "/Game/Blueprints/Widget/WBP_Minimap.WBP_Minimap_C" _returnvalue))
  (`UserWidget.AddToViewport` _returnvalue_6 0)
  (`/Game/Blueprints/Widget/WBP_Minimap.SetMiniRT` _returnvalue_6 (`self.MiniRT`))
  (`KismetSystemLibrary.K2_SetTimer` self "UpdateFog" 0.2 true)
  (`KismetSystemLibrary.K2_SetTimer` self "DrawMinimap" 0.2 true))

(fn `CellIndex`
  (params (Pos :type "Vector Structure"))
  (returns (Index :type Integer))
  (bind _boundsmin (`self.BoundsMin`))
  (bind _cellsize (`self.CellSize`))
  (bind _gridw (`self.GridW`))
  (bind _returnvalue (`KismetMathLibrary.FTrunc` (/ (- (.x Pos) (.x _boundsmin)) _cellsize)))
  (bind _returnvalue_2 (`KismetMathLibrary.FTrunc` (/ (- (.y Pos) (.y _boundsmin)) _cellsize)))
  (if (or (or (< _returnvalue 0) (>= _returnvalue _gridw)) (or (< _returnvalue_2 0) (>= _returnvalue_2 (`self.GridH`))))
    (return -1)
    (else
      (return (+ (* _returnvalue_2 _gridw) _returnvalue)))))

(fn `DrawFog`
  (bind _fogrt (`self.FogRT`))
  (bind _gridw (`self.GridW`))
  (`KismetRenderingLibrary.ClearRenderTarget2D` _fogrt (make `LinearColor` 1.0 1.0 1.0 1.0))
  (bind (_canvas _size _context) (`KismetRenderingLibrary.BeginDrawCanvasToRenderTarget` _fogrt))
  (for _index (range (+ (- (* _gridw (`self.GridH`)) 1) 1))
    (bind _output (`|GetArrayItem` (`self.VisibleHuman`) _index))
    (if (or _output (`|GetArrayItem` (`self.ExploredHuman`) _index))
      (bind _returnvalue (`KismetMathLibrary.FTrunc` (/ (* _index 1.0) _gridw)))
      (`Canvas.K2_DrawTexture` _canvas "/Engine/EngineResources/WhiteSquareTexture.WhiteSquareTexture" (`KismetMathLibrary.MakeVector2D` (* (- _index (* _returnvalue _gridw)) 1.0) (* _returnvalue 1.0)) (`KismetMathLibrary.MakeVector2D` 1.0 1.0) (`KismetMathLibrary.MakeVector2D` 0.0) (`KismetMathLibrary.MakeVector2D` 1.0 1.0) (make `LinearColor` (select `bool` _output :`false` 0.55 :`true` 0.0) 0.0 0.0 1.0) "BLEND_Opaque" 0.0 (`KismetMathLibrary.MakeVector2D` 0.0))))
  (`KismetRenderingLibrary.EndDrawCanvasToRenderTarget` _context))

(fn `DrawMinimap`
  (bind _minirt (`self.MiniRT`))
  (bind _gridw (`self.GridW`))
  (bind _boundsmin (`self.BoundsMin`))
  (bind _cellsize (`self.CellSize`))
  (`KismetRenderingLibrary.ClearRenderTarget2D` _minirt (make `LinearColor` 0.02 0.02 0.03 1.0))
  (bind (_canvas _size _context) (`KismetRenderingLibrary.BeginDrawCanvasToRenderTarget` _minirt))
  (for _index (range (+ (- (* _gridw (`self.GridH`)) 1) 1))
    (bind _output (`|GetArrayItem` (`self.VisibleHuman`) _index))
    (if (or _output (`|GetArrayItem` (`self.ExploredHuman`) _index))
      (bind _returnvalue (`KismetMathLibrary.FTrunc` (/ (* _index 1.0) _gridw)))
      (`Canvas.K2_DrawTexture` _canvas "/Engine/EngineResources/WhiteSquareTexture.WhiteSquareTexture" (`KismetMathLibrary.MakeVector2D` (* (- _index (* _returnvalue _gridw)) 2.0) (* _returnvalue 2.0)) (`KismetMathLibrary.MakeVector2D` 2.0 2.0) (`KismetMathLibrary.MakeVector2D` 0.0) (`KismetMathLibrary.MakeVector2D` 1.0 1.0) (make `LinearColor` (select `bool` _output :`false` 0.28 :`true` 0.55) (select `bool` _output :`false` 0.17 :`true` 0.33) (select `bool` _output :`false` 0.12 :`true` 0.22) 1.0) "BLEND_Opaque" 0.0 (`KismetMathLibrary.MakeVector2D` 0.0))))
  (bind _outactors (`ActorScanner.GetCachedActorsOfClass` "/Game/Blueprints/Units/BP_UnitBase.BP_UnitBase_C"))
  (bind _outactors_2 (`ActorScanner.GetCachedActorsOfClass` "/Game/Blueprints/Buildings/BP_BaseBuilding.BP_BaseBuilding_C"))
  (for _array_element _outactors_2
    (bind _asbp_base_building (cast `/Game/Blueprints/Buildings/BP_BaseBuilding` _array_element))
    (bind _returnvalue_2 (`self.K2_GetActorLocation` _asbp_base_building))
    (bind _index_2 (`self.CellIndex` _returnvalue_2))
    (bind _index_3 (`self.CellIndex` _returnvalue_2))
    (bind _returnvalue_3 (`|EnumEquality` (`/Game/Blueprints/Buildings/BP_BaseBuilding.Faction` _asbp_base_building) (enumliteral `EFaction` "Human")))
    (if (or _returnvalue_3 (`|GetArrayItem` (`self.ExploredHuman`) (select `bool` (< _index_2 0) :`false` _index_3 :`true` 0)))
      (`Canvas.K2_DrawTexture` _canvas "/Engine/EngineResources/WhiteSquareTexture.WhiteSquareTexture" (`KismetMathLibrary.MakeVector2D` (- (* (/ (- (.x _returnvalue_2) (.x _boundsmin)) _cellsize) 2.0) 3.0) (- (* (/ (- (.y _returnvalue_2) (.y _boundsmin)) _cellsize) 2.0) 3.0)) (`KismetMathLibrary.MakeVector2D` 6.0 6.0) (`KismetMathLibrary.MakeVector2D` 0.0) (`KismetMathLibrary.MakeVector2D` 1.0 1.0) (select `bool` _returnvalue_3 :`false` (make `LinearColor` 1.0 0.15 0.1 1.0) :`true` (make `LinearColor` 0.0 0.7 1.0 1.0)) "BLEND_Opaque" 0.0 (`KismetMathLibrary.MakeVector2D` 0.0))))
  (for _array_element_2 _outactors
    (bind _asbp_unit_base (cast `/Game/Blueprints/Units/BP_UnitBase` _array_element_2))
    (bind _bhuman (`/Game/Blueprints/Units/BP_UnitBase.IsHuman` _asbp_unit_base))
    (bind _visible (`self.IsActorVisibleTo` true _asbp_unit_base))
    (if (or _bhuman _visible)
      (bind _returnvalue_4 (`self.K2_GetActorLocation` _asbp_unit_base))
      (`Canvas.K2_DrawTexture` _canvas "/Engine/EngineResources/WhiteSquareTexture.WhiteSquareTexture" (`KismetMathLibrary.MakeVector2D` (- (* (/ (- (.x _returnvalue_4) (.x _boundsmin)) _cellsize) 2.0) 2.0) (- (* (/ (- (.y _returnvalue_4) (.y _boundsmin)) _cellsize) 2.0) 2.0)) (`KismetMathLibrary.MakeVector2D` 4.0 4.0) (`KismetMathLibrary.MakeVector2D` 0.0) (`KismetMathLibrary.MakeVector2D` 1.0 1.0) (select `bool` _bhuman :`false` (make `LinearColor` 1.0 0.3 0.2 1.0) :`true` (make `LinearColor` 0.3 1.0 1.0 1.0)) "BLEND_Opaque" 0.0 (`KismetMathLibrary.MakeVector2D` 0.0))))
  (`KismetRenderingLibrary.EndDrawCanvasToRenderTarget` _context))

(fn `GetNearestUnexplored`
  (params (ForHuman :type Boolean) (From :type "Vector Structure"))
  (returns (Location :type "Vector Structure"))
  (bind _boundsmin (`self.BoundsMin`))
  (bind _cellsize (`self.CellSize`))
  (bind _gridw (`self.GridW`))
  (set `self.ScanBestDist` 1000000000.0)
  (set `self.ScanBestPos` From)
  (for _index (range (+ (- (* _gridw (`self.GridH`)) 1) 1))
    (if (not (select `bool` ForHuman :`false` (`|GetArrayItem` (`self.ExploredAlien`) _index) :`true` (`|GetArrayItem` (`self.ExploredHuman`) _index)))
      (bind _returnvalue (`KismetMathLibrary.FTrunc` (/ (* _index 1.0) _gridw)))
      (bind _returnvalue_2 (`KismetMathLibrary.MakeVector` (+ (.x _boundsmin) (* (+ (- _index (* _returnvalue _gridw)) 0.5) _cellsize)) (+ (.y _boundsmin) (* (+ _returnvalue 0.5) _cellsize))))
      (bind _returnvalue_3 (`KismetMathLibrary.Vector_Distance2D` _returnvalue_2 From))
      (if (and (< _returnvalue_3 (`self.ScanBestDist`)) (> _returnvalue_3 (* _cellsize 2.0)))
        (set `self.ScanBestDist` _returnvalue_3)
        (set `self.ScanBestPos` _returnvalue_2))))
  (return (`self.ScanBestPos`)))

(fn `IsActorVisibleTo`
  (params (ForHuman :type Boolean) (Target :type "Actor Object Reference"))
  (returns (Visible :type Boolean))
  (bind _index (`self.CellIndex` (`self.K2_GetActorLocation` Target)))
  (if (< _index 0)
    (return false)
    (elif ForHuman
      (return (`|GetArrayItem` (`self.VisibleHuman`) _index))
      (else
        (return (`|GetArrayItem` (`self.VisibleAlien`) _index))))))

(fn `MarkSource`
  (params (Pos :type "Vector Structure") (Radius :type "Float (double-precision)") (ForHuman :type Boolean))
  (bind _boundsmin (`self.BoundsMin`))
  (bind _cellsize (`self.CellSize`))
  (bind _gridw (`self.GridW`))
  (bind _returnvalue (+ (`KismetMathLibrary.FTrunc` (/ Radius _cellsize)) 1))
  (for _index (range (- 0 _returnvalue) (+ (- (+ _returnvalue 1) 1) 1))
    (for _index_2 (range (- 0 _returnvalue) (+ (- (+ _returnvalue 1) 1) 1))
      (bind _returnvalue_2 (+ (`KismetMathLibrary.FTrunc` (/ (- (.x Pos) (.x _boundsmin)) _cellsize)) _index_2))
      (bind _returnvalue_3 (+ (`KismetMathLibrary.FTrunc` (/ (- (.y Pos) (.y _boundsmin)) _cellsize)) _index))
      (if (and (and (>= _returnvalue_2 0) (< _returnvalue_2 _gridw)) (and (>= _returnvalue_3 0) (< _returnvalue_3 (`self.GridH`))))
        (if (<= (`KismetMathLibrary.Vector_Distance2D` (`KismetMathLibrary.MakeVector` (+ (.x _boundsmin) (* (+ _returnvalue_2 0.5) _cellsize)) (+ (.y _boundsmin) (* (+ _returnvalue_3 0.5) _cellsize))) Pos) Radius)
          (if ForHuman
            (bind _returnvalue_4 (+ (* _returnvalue_3 _gridw) _returnvalue_2))
            (`KismetArrayLibrary.Array_Set` (`self.VisibleHuman`) _returnvalue_4 true)
            (`KismetArrayLibrary.Array_Set` (`self.ExploredHuman`) _returnvalue_4 true)
            (else
              (`KismetArrayLibrary.Array_Set` (`self.VisibleAlien`) _returnvalue_4 true)
              (`KismetArrayLibrary.Array_Set` (`self.ExploredAlien`) _returnvalue_4 true))))))))

(fn `UpdateFog`
  (for _index (range (+ (- (* (`self.GridW`) (`self.GridH`)) 1) 1))
    (`KismetArrayLibrary.Array_Set` (`self.VisibleHuman`) _index)
    (`KismetArrayLibrary.Array_Set` (`self.VisibleAlien`) _index))
  (bind _outactors (`ActorScanner.GetCachedActorsOfClass` "/Game/Blueprints/Units/BP_UnitBase.BP_UnitBase_C"))
  (bind _outactors_2 (`ActorScanner.GetCachedActorsOfClass` "/Game/Blueprints/Buildings/BP_BaseBuilding.BP_BaseBuilding_C"))
  (for _array_element _outactors
    (bind _asbp_unit_base (cast `/Game/Blueprints/Units/BP_UnitBase` _array_element))
    (bind _bhuman (`/Game/Blueprints/Units/BP_UnitBase.IsHuman` _asbp_unit_base))
    (`self.MarkSource` (`self.K2_GetActorLocation` _asbp_unit_base) (`/Game/Blueprints/Data/PDA_Unit.VisionRadius` (`/Game/Blueprints/Units/BP_UnitBase.Data` _asbp_unit_base)) _bhuman))
  (for _array_element_2 _outactors_2
    (bind _asbp_base_building (cast `/Game/Blueprints/Buildings/BP_BaseBuilding` _array_element_2))
    (`self.MarkSource` (`self.K2_GetActorLocation` _asbp_base_building) 4500.0 (`|EnumEquality` (`/Game/Blueprints/Buildings/BP_BaseBuilding.Faction` _asbp_base_building) (enumliteral `EFaction` "Human"))))
  (for _array_element_3 _outactors
    (bind _asbp_unit_base_2 (cast `/Game/Blueprints/Units/BP_UnitBase` _array_element_3))
    (bind _bhuman_2 (`/Game/Blueprints/Units/BP_UnitBase.IsHuman` _asbp_unit_base_2))
    (if (not _bhuman_2)
      (bind _visible (`self.IsActorVisibleTo` true _asbp_unit_base_2))
      (`self.SetActorHiddenInGame` _asbp_unit_base_2 (not _visible))))
  (for _array_element_4 _outactors_2
    (bind _asbp_base_building_2 (cast `/Game/Blueprints/Buildings/BP_BaseBuilding` _array_element_4))
    (if (not (`|EnumEquality` (`/Game/Blueprints/Buildings/BP_BaseBuilding.Faction` _asbp_base_building_2) (enumliteral `EFaction` "Human")))
      (bind _index_2 (`self.CellIndex` (`self.K2_GetActorLocation` _asbp_base_building_2)))
      (`self.SetActorHiddenInGame` _asbp_base_building_2 (select `bool` (< _index_2 0) :`false` (not (`|GetArrayItem` (`self.ExploredHuman`) _index_2)) :`true` true))))
  (`self.DrawFog`))

(fn `UserConstructionScript`)