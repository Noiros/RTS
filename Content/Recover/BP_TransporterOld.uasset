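; Transporter unit that hauls resources from the mines on its Route to its faction's depots.
; A looping half-second timer replaces Tick logic: when empty, it loads from the current mine and advances the route index, dropping non-mine entries.
; When loaded, it seeks the nearest constructed friendly depot and credits the cargo to the GM_Default faction state.
; AI MoveTo targets and arrival checks allow for building bounds, stopping outside the footprint.
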(event `self.ReceiveBeginPlay`
  (`parent.ReceiveBeginPlay`)
  (`self.StartRoute`))

(event `StartRoute`
  (`KismetSystemLibrary.K2_SetTimer` self "TransportTick" 0.5 true))

(event `TransportTick`
  (bind _bestdepot (`self.BestDepot`))
  (bind _returnvalue (`AIBlueprintHelperLibrary.GetAIController` self))
  (bind _returnvalue_2 (`self.K2_GetActorLocation` self))
  (bind (_origin _boxextent) (`self.GetActorBounds` _bestdepot true false))
  (bind _returnvalue_3 (`self.K2_GetActorLocation` _bestdepot))
  (bind _returnvalue_4 (`KismetMathLibrary.FMax` (.x _boxextent) (.y _boxextent)))
  (if (> (`KismetArrayLibrary.Array_Length` (`self.Route`)) 0)
    (if (== (`self.CarriedAmount`) 0)
      (if (>= (`self.RouteIndex`) (`KismetArrayLibrary.Array_Length` (`self.Route`)))
        (set `self.RouteIndex` 0))
      (bind _asbp_building_mine (cast `/Game/Blueprints/Buildings/BP_Building_Mine` (`|GetArrayItem` (`self.Route`) (`self.RouteIndex`)))
        (:`then`
          (bind (_origin_2 _boxextent_2) (`self.GetActorBounds` _asbp_building_mine true false))
          (bind _returnvalue_5 (`KismetMathLibrary.FMax` (.x _boxextent_2) (.y _boxextent_2)))
          (if (<= (- (`self.GetDistanceTo` self _asbp_building_mine) _returnvalue_5) 250.0)
            (set `self.CarriedAmount` (`KismetMathLibrary.Min` (`/Game/Blueprints/Buildings/BP_Building_Mine.Stock` _asbp_building_mine) (`self.CarryCapacity`)))
            (set `/Game/Blueprints/Buildings/BP_Building_Mine.Stock` (- (`/Game/Blueprints/Buildings/BP_Building_Mine.Stock` _asbp_building_mine) (`self.CarriedAmount`)) _asbp_building_mine)
            (set `self.CarriedResource` (`/Game/Blueprints/Resources/BP_BaseResource.ResourceType` (`/Game/Blueprints/Buildings/BP_Building_Mine.Deposit` _asbp_building_mine)))
            (set `self.RouteIndex` (+ (`self.RouteIndex`) 1))
            (else
              (bind _returnvalue_6 (`self.K2_GetActorLocation` _asbp_building_mine))
              (`AIController.MoveToLocation` _returnvalue (+ _returnvalue_6 (* (`KismetMathLibrary.Normal` (- _returnvalue_2 _returnvalue_6)) (+ _returnvalue_5 120.0))) 50.0 true true false true null true))))
        (:`CastFailed`
          (`KismetArrayLibrary.Array_Remove` (`self.Route`) (`self.RouteIndex`))))
      (else
        (set `self.DepotDist` 1000000.0)
        (bind _outactors (`GameplayStatics.GetAllActorsOfClass` "/Game/Blueprints/Buildings/BP_BaseBuilding.BP_BaseBuilding_C"))
        (for _array_element _outactors
          (bind _bdone (`/Game/Blueprints/Buildings/BP_BaseBuilding.IsConstructed` _array_element))
          (bind _returnvalue_7 (`self.GetDistanceTo` self _array_element))
          (if (and (and _bdone (`/Game/Blueprints/Data/PDA_Building.bIsDepot` (`/Game/Blueprints/Buildings/BP_BaseBuilding.Data` _array_element))) (and (`|EnumEquality` (`/Game/Blueprints/Buildings/BP_BaseBuilding.Faction` _array_element) (`self.Faction`)) (< _returnvalue_7 (`self.DepotDist`))))
            (set `self.DepotDist` _returnvalue_7)
            (set `self.BestDepot` _array_element)))
        (`/Engine/EditorBlueprintResources/StandardMacros.IsValid` _bestdepot
          (:`Is Valid`
            (if (<= (- (`self.GetDistanceTo` self _bestdepot) _returnvalue_4) 250.0)
              (bind _asgm_default (cast `/Game/Blueprints/GM_Default` (`GameplayStatics.GetGameMode`)))
              (bind _state (`/Game/Blueprints/GM_Default.GetFactionState` _asgm_default (`self.Faction`)))
              (`/Game/Blueprints/Core/BP_FactionState.AddResource` _state (`self.CarriedResource`) (`self.CarriedAmount`))
              (set `self.CarriedAmount` 0)
              (else
                (`AIController.MoveToLocation` _returnvalue (+ _returnvalue_3 (* (`KismetMathLibrary.Normal` (- _returnvalue_2 _returnvalue_3)) (+ _returnvalue_4 120.0))) 50.0 true true false true null true)))))))))

(event `self.ReceiveTick`
  (params (DeltaSeconds :type "Float (single-precision)"))
  (`parent.ReceiveTick` DeltaSeconds))

(fn `UserConstructionScript`
  (`parent.UserConstructionScript`))